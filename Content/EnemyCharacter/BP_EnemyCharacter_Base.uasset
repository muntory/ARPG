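; Base enemy character Blueprint that handles death with a dissolve effect before removing the enemy.
; On death it freezes the mesh animation, disables capsule collision and async-loads the supplied Niagara system, attaching it to the mesh with a color read from a dynamic material instance.
; A timeline, rate-scaled by the total dissolve time, drives the dissolve parameter on body and equipped weapon materials, then destroys both actors.
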(event EventBeginPlay)

(event Collision|EventActorBeginOverlap
  (params (OtherActor :type Actor%20Object%20Reference)))

(event EventOnEnemyDied
  (params (DissolveNiagaraSystem :type Niagara%20System%20Soft%20Object%20Reference))
  (bind _mesh (Variables|Character|GetMesh))
  (bind _enemycombatcomponent (Variables|Default|GetEnemyCombatComponent))
  (bind _returnvalue (Class|ARPGPawnCombatComponent|GetCurrentEquippingWeapon _enemycombatcomponent))
  (Utilities|FlowControl|Sequence
    (:then_0
      (Variables|/Script/Engine.SkeletalMeshComponent|SetbPauseAnims (Variables|Character|GetMesh) true)
      (Collision|SetCollisionEnabled (Variables|Default|GetCapsuleComponent) "NoCollision"))
    (:then_1
      (bind _object (Utilities|AsyncLoadAsset DissolveNiagaraSystem)
        (:Completed
          (bind _asniagara_system (Utilities|Casting|CastToNiagaraSystem _object))
          (bind _returnvalue_2 (Niagara|SpawnSystemAttached _asniagara_system (Variables|Character|GetMesh) "None" "0, 0, 0" "0, 0, 0" "KeepRelativeOffset" true))
          (bind _returnvalue_3 (Rendering|Material|CreateDynamicMaterialInstance _mesh 0 (Rendering|Material|GetMaterial _mesh 0) "DissolveEdgeColor" :!class /Script/Engine.PrimitiveComponent))
          (bind _returnvalue_4 (Rendering|Material|GetVectorParameterValue _returnvalue_3 "None" :!class /Script/Engine.MaterialInstanceDynamic))
          (Niagara|SetNiagaraVariable(LinearColor) _returnvalue_2 "DissolveParticleColor" _returnvalue_4)
          (Components|Timeline|SetPlayRate (Variables|Default|GetDissolveTimeline) (/ 1.0 (Variables|Default|GetTotalDissolveTime)))
          (bind _normalizedfloattrack (Timeline|DissolveTimeline PlayFromStart)
            (:Update
              (Rendering|Material|SetScalarParameterValueonMaterials (Variables|Character|GetMesh) "DissolveAmount" _normalizedfloattrack)
              (Utilities|IsValid (Class|ARPGPawnCombatComponent|GetCurrentEquippingWeapon (Variables|Default|GetEnemyCombatComponent))
                (:Is%20Valid
                  (Rendering|Material|SetScalarParameterValueonMaterials (Variables|/Script/ARPG.ARPGBaseWeapon|GetWeaponMesh (Class|ARPGPawnCombatComponent|GetCurrentEquippingWeapon (Variables|Default|GetEnemyCombatComponent))) "DissolveAmount" _normalizedfloattrack))))
            (:Finished
              (Utilities|IsValid _returnvalue
                (:Is%20Valid
                  (Actor|DestroyActor _returnvalue))
                (:Is%20Not%20Valid
                  _))
              (Actor|DestroyActor))))))))

(fn ConstructionScript)